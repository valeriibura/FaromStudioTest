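; Pong-style ball pawn that launches in a random diagonal on BeginPlay and feeds its velocity into FloatingPawnMovement every Tick.
; Sphere overlaps flip X on walls; on BP_Player they flip Y, add the player's normalized X velocity and scale max speed by SpeedMultipy.
; Hitting a BP_GoalField spawns a replacement ball, increments the matching score on BP_AGameModeBase and destroys this one.
; Line-trace reflection debug logic is left unconnected.
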(event OnComponentBeginOverlap(SphereCollision)
  (params (OverlappedComponent :type Primitive%20Component%20Object%20Reference) (OtherActor :type Actor%20Object%20Reference) (OtherComp :type Primitive%20Component%20Object%20Reference) (OtherBodyIndex :type Integer) (bFromSweep :type Boolean) (SweepResult :type Hit%20Result%20Structure%20%28by%20ref%29))
  (bind _floatingpawnmovement (Variables|Default|GetFloatingPawnMovement))
  ;[1 1 1] Console
  (Utilities|Casting|CastToBP_Wall OtherActor
    (:then
      (Development|PrintString "Wall")
      (Variables|Default|SetVelocity (Math|Vector|MakeVector (* (.x (Variables|Default|GetVelocity)) -1.0) (.y (Variables|Default|GetVelocity)) (.z (Variables|Default|GetVelocity)))))
    (:CastFailed
      (bind _asbp_player (Utilities|Casting|CastToBP_Player OtherActor)
        (:then
          (Development|PrintString "Player")
          (Variables|Default|SetVelocity (Math|Vector|MakeVector (+ (.x (Variables|Default|GetVelocity)) (/ (.x (Transformation|GetVelocity _asbp_player)) (Class|MovementComponent|GetMaxSpeed (Variables|/Script/Engine.Character|GetCharacterMovement _asbp_player)))) (* (.y (Variables|Default|GetVelocity)) -1.0) (.z (Variables|Default|GetVelocity))))
          (Variables|/Script/Engine.FloatingPawnMovement|SetMaxSpeed _floatingpawnmovement (* (Class|MovementComponent|GetMaxSpeed _floatingpawnmovement) (Variables|Default|GetSpeedMultipy))))
        (:CastFailed
          (bind _asbp_goal_field (Utilities|Casting|CastToBP_GoalField OtherActor))
          (CallFunction|Goal (Variables|/Game/Blueprints/BP_GoalField.BP_GoalField_C|GetPlayerTargetGoal _asbp_goal_field))
          (Actor|DestroyActor))))))

(event Custom|Goal
  (params (PlayerGoal :type Boolean))
  ;[1 1 1] SpawnBall
  (Game|SpawnActorfromClass "BP_AActor_C" (Math|Transform|MakeTransform "30.000000,70.000000,0.000000") "Undefined" 0 0)
  (bind _asbp_agame_mode_base (Utilities|Casting|CastToBP_AGameModeBase (Game|GetGameMode)))
  (Math|Integer|IncrementInt (select PlayerGoal (Variables|/Game/Blueprints/BP_AGameModeBase.BP_AGameModeBase_C|GetPlayerScore _asbp_agame_mode_base) (Variables|/Game/Blueprints/BP_AGameModeBase.BP_AGameModeBase_C|GetOtherPlayerScore _asbp_agame_mode_base))
    (:%20%20
      (Actor|DestroyActor))))

(event EventBeginPlay
  ;[1 1 1] Movement
  (Variables|Default|SetVelocity (Math|Vector|MakeVector (select (Math|Random|RandomBool) 1.0 -1.0) (select (Math|Random|RandomBool) 1.0 -1.0) 0.0)))

(event EventTick
  (params (DeltaSeconds :type Float%20%28single-precision%29))
  ;[1 1 1] Line Trace
  (Class|PawnMovementComponent|AddInputVector (Variables|Default|GetFloatingPawnMovement) (Variables|Default|GetVelocity) false))

(fn ConstructionScript)