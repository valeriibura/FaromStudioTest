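; BP_Player is the player actor, confined to a fixed band along the world X axis.
; Each Tick checks the actor's X position and snaps it back to the nearer limit when outside, leaving Y and Z unchanged.
; After an in-range check or an upper-limit snap, execution order is not branched further except for a debug print of X velocity relative to CharacterMovement's max speed.
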(event EventTick
  (params (DeltaSeconds :type Float%20%28single-precision%29))
  (bind _returnvalue (Transformation|GetActorLocation))
  ;[1 1 1] Block Player
  (if (> (.x _returnvalue) 3.3e+02)
    (Transformation|SetActorLocation (Math|Vector|MakeVector 3.3e+02 (.y _returnvalue) (.z _returnvalue)) false false)
    (elif (< (.x _returnvalue) -3e+02)
      (Transformation|SetActorLocation (Math|Vector|MakeVector -3e+02 (.y _returnvalue) (.z _returnvalue)) false false)))
  (Development|PrintString (Utilities|String|ToString(Float) (/ (.x (Transformation|GetVelocity)) (Class|MovementComponent|GetMaxSpeed (Variables|Character|GetCharacterMovement)))) true true "(R=0.000000,G=1.000000,B=0.227042,A=1.000000)" 0.0))

(fn ConstructionScript)